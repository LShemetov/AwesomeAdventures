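; Player controller that possesses the level's BP_PlayerShip on BeginPlay and lets the player place a click marker in the world.
; A left click deprojects the mouse position and line-traces along it on the Visibility channel.
; On a hit it destroys the previous marker and spawns a new BP_Marker at the hit point, so only one exists at a time.
; CheckSpawnMarkerPosibility is an empty stub.
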(event `self.ReceiveBeginPlay`
  (bind _returnvalue (`GameplayStatics.GetActorOfClass` "/Game/Blueprints/Ships/BP_PlayerShip.BP_PlayerShip_C"))
  (bind _output_get (set `self.PlayerShip` _returnvalue))
  (`self.Possess` _output_get))

(event `Key|LeftMouseButton`
  (params (Key :type "Key Structure"))
  (bind (_worldlocation _worlddirection) (`self.DeprojectMousePositionToWorld`))
  (:`Pressed`
    (bind (_outhit _returnvalue) (`KismetSystemLibrary.LineTraceSingle` :`Start` _worldlocation :`End` (+ _worldlocation (* _worlddirection 100000.0)) :`TraceChannel` "TraceTypeQuery1" :`DrawTime` 0.5))
    (if _returnvalue
      (bind _activemarker (`self.ActiveMarker`)
        (:`then`
          (`self.K2_DestroyActor` _activemarker))
        (:`else`
          _))
      (bind _returnvalue_2 (`|SpawnActorFromClass` "/Game/Blueprints/Navigation/BP_Marker.BP_Marker_C" (`KismetMathLibrary.MakeTransform` (`.Location` (`GameplayStatics.BreakHitResult` _outhit))) "Undefined" "MultiplyWithRoot" null null))
      (set `self.ActiveMarker` _returnvalue_2))))

(fn `CheckSpawnMarkerPosibility`)

(fn `UserConstructionScript`)