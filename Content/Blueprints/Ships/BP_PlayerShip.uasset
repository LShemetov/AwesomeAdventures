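; BP_PlayerShip is a player ship that turns toward and sails after an assigned target actor.
; While motion is enabled and a target is valid, Tick yaws the ship at constant speed, then moves it forward in XY.
; A dot product with the right vector picks turn direction when the target is set.
; Yaw snaps to the look-at angle once within one step, then stops updating.
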(event `self.ReceiveTick`
  (params (DeltaSeconds :type "Float (single-precision)"))
  (bind _returnvalue (`self.K2_GetActorLocation`))
  (bind (_returnvalue_roll _returnvalue_pitch _returnvalue_yaw) (`KismetMathLibrary.BreakRotator` (`self.K2_GetActorRotation`)))
  (bind (_returnvalue_roll_2 _returnvalue_pitch_2 _returnvalue_yaw_2) (`KismetMathLibrary.BreakRotator` (`KismetMathLibrary.FindLookAtRotation` (`self.K2_GetActorLocation`) (`self.K2_GetActorLocation` (`self.CurrentTarget`)))))
  (bind (_returnvalue_roll_3 _returnvalue_pitch_3 _returnvalue_yaw_3) (`KismetMathLibrary.BreakRotator` (`KismetMathLibrary.FindLookAtRotation` (`self.K2_GetActorLocation`) (`self.K2_GetActorLocation` (`self.CurrentTarget`)))))
  (bind (_returnvalue_x _returnvalue_y) (`KismetMathLibrary.BreakVector` (* (`self.GetActorForwardVector`) (* (`self.MotionSpeed`) (`self.DeltaSeconds`)))))
  (set `self.DeltaSeconds` DeltaSeconds)
  (`|ExecutionSequence`
    (:`then_0`
      (`KismetSystemLibrary.DrawDebugArrow` _returnvalue (+ _returnvalue (* (`self.GetActorForwardVector`) 20000.0)) 0.0 (struct :`R` 1.0 :`G` 0.007402 :`A` 1.0)))
    (:`then_1`
      (if (`self.bIsMotionAvailable`)
        (bind _currenttarget (`self.CurrentTarget`)
          (:`then`
            (`|ExecutionSequence`
              (:`then_0`
                (`KismetSystemLibrary.DrawDebugArrow` (`self.K2_GetActorLocation`) (`self.K2_GetActorLocation` _currenttarget) 70.0 (struct :`G` 0.255457 :`B` 1.0 :`A` 1.0)))
              (:`then_1`
                (if (`self.bIsRotationReached`)
                  _
                  (elif (<= (`KismetMathLibrary.Abs` (- _returnvalue_yaw_3 _returnvalue_yaw)) (`KismetMathLibrary.Abs` (`self.CalcDeltaRotation`)))
                    (`self.K2_SetActorRotation` (`KismetMathLibrary.MakeRotator` 0.0 0.0 _returnvalue_yaw_2))
                    (set `self.bIsRotationReached` true)
                    (else
                      (`self.K2_AddActorWorldRotation` (`KismetMathLibrary.MakeRotator` 0.0 0.0 (`self.CalcDeltaRotation`)))))))
              (:`then_2`
                (`self.K2_AddActorWorldOffset` (`KismetMathLibrary.MakeVector` _returnvalue_x _returnvalue_y)))))
          (:`else`))))))

(fn `CalcAngleWithTarget`
  (returns (Angle :type "Float (double-precision)"))
  (return (`KismetMathLibrary.DegAcos` (`KismetMathLibrary.Dot_VectorVector` (`self.GetActorForwardVector`) (`KismetMathLibrary.Normal` (- (`self.K2_GetActorLocation` (`self.CurrentTarget`)) (`self.K2_GetActorLocation`)) 1e-06)))))

(fn `CalcDeltaRotation`
  (returns (DeltaRotation :type "Float (double-precision)"))
  (return (* (`self.RotationSign`) (`self.RotationSpeed`) (`self.DeltaSeconds`))))

(fn `CalcNewMotionTargetParameters`
  (params (InTarget :type "Actor Object Reference"))
  (`self.SetMotionTarget` InTarget)
  (`self.CalcRotationSign`)
  (`self.CalcTargetRotation`)
  (set `self.bIsRotationReached` false))

(fn `CalcRotationSign`
  (set `self.RotationSign` (`KismetMathLibrary.SignOfFloat` (`KismetMathLibrary.Dot_VectorVector` (`self.GetActorRightVector`) (`KismetMathLibrary.Normal` (- (`self.K2_GetActorLocation` (`self.CurrentTarget`)) (`self.K2_GetActorLocation`)) 1e-06)))))

(fn `CalcTargetRotation`
  (bind (_returnvalue_roll _returnvalue_pitch _returnvalue_yaw) (`KismetMathLibrary.BreakRotator` (`self.K2_GetActorRotation`)))
  (set `self.TargetRotation` (`KismetMathLibrary.MakeRotator` _returnvalue_roll _returnvalue_pitch (+ _returnvalue_yaw (* (`self.CalcAngleWithTarget`) (`self.RotationSign`))))))

(fn `ClearMotionTarget`
  (set `self.CurrentTarget` null))

(fn `DisableMotion`
  (set `self.bIsMotionAvailable` false))

(fn `EnableMotion`
  (set `self.bIsMotionAvailable` true))

(fn `SetMotionTarget`
  (params (InTarget :type "Actor Object Reference"))
  (set `self.CurrentTarget` InTarget))

(fn `UserConstructionScript`
  (`parent.UserConstructionScript`))