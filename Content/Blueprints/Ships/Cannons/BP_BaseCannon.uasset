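; Base ship cannon that automatically fires whenever its Target is valid and in its firing arc.
; Each Tick it checks that the target is within FireAngle of the actor's forward vector, within FireDistance, and that the cannon is not reloading.
; Fire only starts the reload state, with no projectile or damage logic here; a named-function timer clears it after ReloadTime.
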(event `self.ReceiveTick`
  (params (DeltaSeconds :type "Float (single-precision)"))
  (`self.Target`
    (:`then`
      (if (`self.CheckFirePosibility`)
        (`self.Fire`)))
    (:`else`)))

(fn `CheckFirePosibility`
  (returns (bIsFirePossible :type Boolean))
  (locals (SightVector :type "Vector Structure"))
  (bind _output_get (set `local.SightVector` (- (`self.K2_GetActorLocation` (`self.Target`)) (`self.K2_GetActorLocation`))))
  (return (and (<= (`KismetMathLibrary.DegAcos` (`KismetMathLibrary.Dot_VectorVector` (`KismetMathLibrary.Normal` _output_get) (`self.GetActorForwardVector`))) (`self.FireAngle`)) (<= (`KismetMathLibrary.VSize` (`local.SightVector`)) (`self.FireDistance`)) (not (`self.bIsOnReaload`)))))

(fn `Fire`
  (set `self.bIsOnReaload` true)
  (`self.StartReloadTimer`))

(fn `Reload`
  (set `self.bIsOnReaload` false))

(fn `StartReloadTimer`
  (bind _returnvalue (`KismetSystemLibrary.K2_SetTimer` null "Reload" (`self.ReloadTime`)))
  (set `self.ReloadTimer` _returnvalue))

(fn `UserConstructionScript`)